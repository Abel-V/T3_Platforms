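; Movable platform actor that travels along a timeline-driven offset from the location it records at BeginPlay.
; Tick calls Play on the timeline, whose update scales its track output by Distancia, adds it to the start position and sets the actor location without sweep.
; The Horizontal flag swaps the offset's Y and Z components, redirecting the same motion curve onto another axis.
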(event `self.ReceiveBeginPlay`
  (bind _output_get (set `self.PosicionInicial` (`self.K2_GetActorLocation`))))

(event `self.ReceiveTick`
  (params (DeltaSeconds :type "Float (single-precision)"))
  (bind (_direction _newtrack_0) (`Timeline|Timeline_0`)
    (:`Update`
      (if (`self.Horizontal`)
        (bind _returnvalue (* _newtrack_0 (`self.Distancia`)))
        (`self.K2_SetActorLocation` (+ (`self.PosicionInicial`) (`KismetMathLibrary.MakeVector` (.x _returnvalue) (.z _returnvalue) (.y _returnvalue))))
        (else
          (`self.K2_SetActorLocation` (+ (stale `self.ReceiveBeginPlay` _output_get) _returnvalue)))))))

(fn `UserConstructionScript`)
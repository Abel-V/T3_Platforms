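; Elevator actor that moves from its starting location along a configurable Distancia offset when F is pressed.
; It caches its location on BeginPlay, then a timeline curve scales the offset and sets the actor's position each update, without sweep.
; The Horizontal flag swaps the offset's Y and Z components to turn vertical travel sideways.
; When the timeline finishes, its playback time is reset.
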(event `self.ReceiveBeginPlay`
  (bind _output_get (set `self.PosicionInicial` (`self.K2_GetActorLocation`))))

(event `Key|F`
  (params (Key :type "Key Structure"))
  (:`Pressed`
    (bind (_direction _newtrack_0) (`Timeline|Timeline_0` :!label _label)
      (:`Update`
        (if (`self.Horizontal`)
          (bind _returnvalue (* _newtrack_0 (`self.Distancia`)))
          (`self.K2_SetActorLocation` (+ (`self.PosicionInicial`) (`KismetMathLibrary.MakeVector` (.x _returnvalue) (.z _returnvalue) (.y _returnvalue))))
          (else
            (`self.K2_SetActorLocation` (+ (stale `self.ReceiveBeginPlay` _output_get) _returnvalue)))))
      (:`Finished`
        (goto _label :!via `SetNewTime`)))))

(fn `UserConstructionScript`)